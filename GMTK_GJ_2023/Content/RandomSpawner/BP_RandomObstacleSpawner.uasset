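; BP_RandomObstacleSpawner rolls a random chance to spawn an obstacle on a looping timer set to MinTime from BeginPlay.
; Each failed roll raises CurrentChance by a fixed step, capped at Maxchance, so success grows likelier.
; A successful roll resets the chance to a base that rises linearly over the first five minutes of game time.
; The spawn itself is only a placeholder comment; no obstacle is created.
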(event `self.ReceiveBeginPlay`
  (`KismetSystemLibrary.K2_SetTimerDelegate` (delegate `SpawnObstacleChance`) (`self.MinTime`) true))

(event `SpawnObstacleChance`
  (if (<= (`KismetMathLibrary.RandomFloatInRange` 0.0 1.0) (`self.CurrentChance`))
    ;[1 1 1] Reset current chance to base chance and spawn an obstacle here
    (set `self.CurrentChance` (/ (`KismetMathLibrary.FClamp` (`KismetSystemLibrary.GetGameTimeInSeconds`) 0.0 300.0) 1000.0))
    (else
      ;[1 1 1] Increment current chance if not spawning platform. Clamp between 0 and maxchance
      (set `self.CurrentChance` (`KismetMathLibrary.FClamp` (+ (`self.CurrentChance`) 0.1) 0.0 (`self.Maxchance`))))))

(fn `UserConstructionScript`)