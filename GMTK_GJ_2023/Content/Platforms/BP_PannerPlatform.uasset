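; BP_PannerPlatform is a platform that scrolls steadily along negative world Y and records when the player has passed it.
; Tick offsets the whole actor by a fixed step each frame, unscaled by delta time.
; BeginPlay caches the BP_Player and BP_LevelPanner actors, though the panner reference is unused in these graphs.
; Player overlap with the box sets PlatformPassed and prints it for debugging.
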(event `self.ReceiveBeginPlay`
  (bind _returnvalue (`GameplayStatics.GetActorOfClass` "/Game/Player/BP_Player.BP_Player_C"))
  (set `self.PlayerRef` _returnvalue)
  (bind _returnvalue_2 (`GameplayStatics.GetActorOfClass` "/Game/Platforms/BP_LevelPanner.BP_LevelPanner_C"))
  (set `self.LevelPanner` _returnvalue_2))

(event `self.ReceiveTick`
  (params (DeltaSeconds :type "Float (single-precision)"))
  (`self.K2_AddActorWorldOffset` (0.0 -10.0 0.0)))

(event `self.Box_0.OnComponentBeginOverlap`
  (params (OverlappedComponent :type "PrimitiveComponent Object Reference") (OtherActor :type "Actor Object Reference") (OtherComp :type "PrimitiveComponent Object Reference") (OtherBodyIndex :type Integer) (bFromSweep :type Boolean) (SweepResult :type "HitResult Structure (by ref)"))
  (if (== OtherActor (`self.PlayerRef`))
    (bind _output_get (set `self.PlatformPassed` true))
    (`KismetSystemLibrary.PrintString` (`KismetStringLibrary.Conv_BoolToString` _output_get))))

(fn `UserConstructionScript`
  (`parent.UserConstructionScript`))