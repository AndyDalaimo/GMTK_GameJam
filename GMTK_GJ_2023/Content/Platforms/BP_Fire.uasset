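; BP_Fire is a fire hazard actor that cooks the player on contact.
; On BeginPlay it finds and caches the BP_Player actor.
; When that player begins overlapping its Box component, it calls CookPlayer on the player with a fixed amount.
; An older direct decrement of the player's Cooked value with a debug print remains disconnected.
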(event `self.ReceiveBeginPlay`
  (bind _returnvalue (`GameplayStatics.GetActorOfClass` "/Game/Player/BP_Player.BP_Player_C"))
  (set `self.PlayerRef` _returnvalue))

(event `self.Box.OnComponentBeginOverlap`
  (params (OverlappedComponent :type "PrimitiveComponent Object Reference") (OtherActor :type "Actor Object Reference") (OtherComp :type "PrimitiveComponent Object Reference") (OtherBodyIndex :type Integer) (bFromSweep :type Boolean) (SweepResult :type "HitResult Structure (by ref)"))
  (if (== OtherActor (`self.PlayerRef`))
    (`/Game/Player/BP_Player.CookPlayer` (`self.PlayerRef`) 10.0)))

(fn `UserConstructionScript`)