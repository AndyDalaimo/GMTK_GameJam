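; BP_Panner recycles platform actors along the Y axis to keep a repeating track under the player.
; BeginPlay caches all BP_PannerPlatform actors and the BP_Player, deriving platform length from the first cube's bounds and scale.
; Each Tick, any platform at least two lengths behind the player in Y jumps forward by the whole row's length.
; An older destroy-and-spawn approach remains disconnected, and debug prints are left in.
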(event `self.ReceiveBeginPlay`
  (bind _cube (`/Game/Platforms/BP_PannerPlatform.Cube` (`|GetArrayItem` (`self.PlatformRefs`))))
  (bind (_min _max) (`StaticMeshComponent.GetLocalBounds` _cube))
  (bind (_relativescale3d_x _relativescale3d_y) (`KismetMathLibrary.BreakVector` (`SceneComponent.RelativeScale3D` _cube)))
  (bind (_returnvalue_x _returnvalue_y) (`KismetMathLibrary.BreakVector` (- _max _min)))
  (bind _outactors (`GameplayStatics.GetAllActorsOfClass` "/Game/Platforms/BP_PannerPlatform.BP_PannerPlatform_C"))
  (set `self.PlatformRefs` _outactors)
  (bind _returnvalue (`GameplayStatics.GetActorOfClass` "/Game/Player/BP_Player.BP_Player_C"))
  (set `self.PlayerRef` _returnvalue)
  (bind _output_get (set `self.PlatformLength` (* _relativescale3d_y _returnvalue_y)))
  (`KismetSystemLibrary.PrintString` (`KismetStringLibrary.Conv_DoubleToString` _output_get)))

(event `self.ReceiveTick`
  (params (DeltaSeconds :type "Float (single-precision)"))
  (for _array_element (`self.PlatformRefs`)
    (bind (_returnvalue_x _returnvalue_y) (`KismetMathLibrary.BreakVector` (- (`self.K2_GetActorLocation` (`self.PlayerRef`)) (`self.K2_GetActorLocation` _array_element))))
    (if (>= _returnvalue_y (* (`self.PlatformLength`) 2.0))
      (`KismetSystemLibrary.PrintString` "YES")
      (`self.K2_AddActorWorldOffset` _array_element (`KismetMathLibrary.MakeVector` 0.0 (* (`self.PlatformLength`) (`KismetArrayLibrary.Array_Length` (`self.PlatformRefs`)))) false false))))

(event `self.Box.OnComponentEndOverlap`
  (params (OverlappedComponent :type "PrimitiveComponent Object Reference") (OtherActor :type "Actor Object Reference") (OtherComp :type "PrimitiveComponent Object Reference") (OtherBodyIndex :type Integer)))

(fn `UserConstructionScript`)