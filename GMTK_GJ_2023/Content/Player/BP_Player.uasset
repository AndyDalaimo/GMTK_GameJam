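; Player Blueprint for a side-scrolling, cooking-themed launch game, moving a physics cube along Y with a fixed-height camera and a velocity clamp.
; Holding left mouse slows time, shows a direction actor and plays the spatula animation; release converts the drag into an impulse, then a timeline recharges the launch.
; Right mouse spends condiment pickups through BP_PowerupHandler.
; Pickups, score, cooked level and cooldown feed WBP_HUD.
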(event `self.ReceiveBeginPlay`
  (set `self.CameraLoc` (`SceneComponent.K2_GetComponentLocation` (`self.Camera`)))
  (bind _returnvalue (`GameplayStatics.GetActorOfClass` "/Game/Player/Powerups/BP_PowerupHandler.BP_PowerupHandler_C"))
  (set `self.PowerUpHandler` _returnvalue)
  (bind _asplayer_controller (cast `PlayerController` (`self.GetController`)))
  (bind _returnvalue_2 (`|CreateWidget` "/Game/UI/WBP_HUD.WBP_HUD_C" _asplayer_controller))
  (bind _output_get (set `self.HUD` _returnvalue_2))
  (`UserWidget.AddToViewport` _output_get 0)
  (`/Game/UI/WBP_HUD.UpdateCondimentUI` _output_get (`self.Pickups`)))

(event `self.ReceiveTick`
  (params (DeltaSeconds :type "Float (single-precision)"))
  (bind _camera (`self.Camera`))
  (bind (_cameraloc_x _cameraloc_y _cameraloc_z) (`KismetMathLibrary.BreakVector` (`self.CameraLoc`)))
  (bind (_returnvalue_x _returnvalue_y) (`KismetMathLibrary.BreakVector` (`SceneComponent.K2_GetComponentLocation` _camera)))
  (`SceneComponent.K2_AddWorldOffset` (`self.Cube`) (0.0 6.0 0.0) false true)
  (if (not (`self.isFiring`))
    (`SceneComponent.K2_SetWorldLocation` _camera (`KismetMathLibrary.MakeVector` _cameraloc_x _returnvalue_y _cameraloc_z) false false)
    (`self.ClampPlayerVelo`)))

(event `Key|LeftMouseButton`
  (params (Key :type "Key Structure"))
  (bind (_launchpower_x _launchpower_y) (`KismetMathLibrary.BreakVector2D` (`self.LaunchPower`)))
  (bind (_locationx _locationy) (`PlayerController.GetMousePosition` (`GameplayStatics.GetPlayerController` 0)))
  (:`Pressed`
    (if (== (`self.LaunchTimer`) 1.0)
      (set `self.isFiring` true)
      (`GameplayStatics.SetGlobalTimeDilation` 0.2)
      (set `self.InitMousePos` (`KismetMathLibrary.MakeVector2D` _locationx _locationy))
      (bind _returnvalue (`|SpawnActorFromClass` "/Game/Player/BP_LaunchDirection.BP_LaunchDirection_C" (`KismetMathLibrary.MakeTransform` (`SceneComponent.K2_GetComponentLocation` (`self.LaunchDir`)) (struct :`Yaw` 90.0)) "Undefined" "OverrideRootScale" null null))
      (set `self.LaunchDirRef` _returnvalue)
      (`PaperFlipbookComponent.SetPlayRate` (`/Game/Player/Powerups/BP_PowerupHandler.Spatula` (`self.PowerUpHandler`)) 1.0)))
  (:`Released`
    (if (and (== (`self.LaunchTimer`) 1.0) (`self.isFiring`))
      (`self.SetLaunchPower`)
      (`PrimitiveComponent.AddImpulse` (`self.Cube`) (`KismetMathLibrary.MakeVector` 0.0 _launchpower_x _launchpower_y) "None" true)
      (set `self.isFiring` false)
      (`self.ResetSpatulaAnim`)
      (`self.LaunchDirHandler`)
      (bind (_direction _time) (`Timeline|Launch` :!via `PlayFromStart`)
        (:`Update`
          (`self.LaunchTimerHandler` _time))))))

(event `Key|RightMouseButton`
  (params (Key :type "Key Structure"))
  (:`Pressed`
    (if (> (`self.Pickups`) 0)
      (`/Game/Player/Powerups/BP_PowerupHandler.DropPowerup` (`self.PowerUpHandler`))
      (bind _result (`/Engine/EditorBlueprintResources/StandardMacros.DecrementInt` (`self.Pickups`))
        (:`  `
          (`/Game/UI/WBP_HUD.UpdateCondimentUI` (`self.HUD`) _result))))))

(fn `ClampPlayerVelo`
  (bind _maxvelo (`self.MaxVelo`))
  (bind _cube (`self.Cube`))
  (bind (_returnvalue_x _returnvalue_y) (`KismetMathLibrary.BreakVector` (`SceneComponent.GetComponentVelocity` (`self.Cube`))))
  (bind (_returnvalue_x_2 _returnvalue_y_2 _returnvalue_z) (`KismetMathLibrary.BreakVector` (`SceneComponent.GetComponentVelocity` _cube)))
  (if (>= _returnvalue_y _maxvelo)
    (bind _returnvalue (`KismetMathLibrary.FloatSpringInterp` _maxvelo 400.0 (make `FloatSpringState`) 0.0 0.0 1.2))
    (`PrimitiveComponent.SetPhysicsLinearVelocity` _cube (`KismetMathLibrary.MakeVector` 0.0 _returnvalue _returnvalue_z) false "None")))

(fn `CookPlayer`
  (params (Amount :type "Float (double-precision)"))
  (bind _hud (`self.HUD`))
  (bind _output_get (set `self.Cooked` (+ (`self.Cooked`) Amount)))
  (`/Game/UI/WBP_HUD.UpdateCookometer` _hud (/ _output_get 100.0))
  (`UserWidget.PlayAnimation` _hud (`/Game/UI/WBP_HUD.CookOMeterUpdated` _hud) 0.0 1 "Forward" 1.0 false))

(fn `GainPickup`
  (bind _result (`/Engine/EditorBlueprintResources/StandardMacros.IncrementInt` (`self.Pickups`))
    (:`  `
      (bind _output_get (set `self.Pickups` (`KismetMathLibrary.Clamp` _result 0 3)))
      (`/Game/UI/WBP_HUD.UpdateCondimentUI` (`self.HUD`) _output_get)
      (if (== (`self.Pickups`) 3)
        (`self.IncreaseScore` 50)
        (else
          (`self.IncreaseScore` 25))))))

(fn `IncreaseScore`
  (params (Amount :type Integer))
  (bind _output_get (set `self.Score` (+ (`self.Score`) Amount)))
  (`/Game/UI/WBP_HUD.UpdateScoreUI` (`self.HUD`) _output_get))

(fn `LaunchTimerHandler`
  (params (LaunchTimer :type "Float (double-precision)"))
  (bind _hud (`self.HUD`))
  (set `self.LaunchTimer` LaunchTimer)
  ;[1 1 1 0] Update UI Here
  (`ProgressBar.SetPercent` (`/Game/UI/WBP_HUD.PB_LaunchTimer` (`self.HUD`)) (/ (`self.LaunchTimer`) 1.0))
  (if (> (`self.LaunchTimer`) 0.95)
    (`UserWidget.PlayAnimation` _hud (`/Game/UI/WBP_HUD.LaunchTimerReady` _hud) 0.0 1 "Forward" 1.0 false)))

(fn `SetLaunchPower`
  (bind (_locationx _locationy) (`PlayerController.GetMousePosition` (`GameplayStatics.GetPlayerController` 0)))
  (bind (_returnvalue_x _returnvalue_y) (`KismetMathLibrary.BreakVector2D` (* (`self.FinalMousePos`) (-10.0 10.0))))
  (set `self.FinalMousePos` (- (`KismetMathLibrary.MakeVector2D` _locationx _locationy) (`self.InitMousePos`)))
  (set `self.LaunchPower` (`KismetMathLibrary.MakeVector2D` (`KismetMathLibrary.FClamp` _returnvalue_x 0.0 550.0) (`KismetMathLibrary.FClamp` _returnvalue_y 0.0 1000.0)))
  (return))

(fn `UserConstructionScript`)