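; BP_Pickup is a collectible that drifts along the world Y axis and rewards the player on contact.
; On BeginPlay it picks a random sprite and negative speed, then a looping timer moves it in place of Tick.
; Overlapping the cached BP_Player reference calls GainPickup and destroys the pickup, while a second timer destroys it after a fixed lifetime.
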(event `self.ReceiveBeginPlay`
  (bind _returnvalue (`GameplayStatics.GetActorOfClass` "/Game/Player/BP_Player.BP_Player_C"))
  (set `self.PlayerRef` _returnvalue)
  (`PaperSpriteComponent.SetSprite` (`self.Sprite`) (`|GetArrayItem` (`self.SpriteArray`) (`KismetMathLibrary.RandomInteger` 3)))
  (set `self.Speed` (`KismetMathLibrary.RandomFloatInRange` -10.0 -25.0))
  (`KismetSystemLibrary.K2_SetTimerDelegate` (delegate `Move`) 0.05 true)
  (`KismetSystemLibrary.K2_SetTimerDelegate` (delegate `Destroy`) 10.0))

(event `Destroy`
  (`self.K2_DestroyActor`))

(event `Move`
  (`self.K2_AddActorWorldOffset` (`KismetMathLibrary.MakeVector` 0.0 (`self.Speed`))))

(event `self.Collider.OnComponentBeginOverlap`
  (params (OverlappedComponent :type "PrimitiveComponent Object Reference") (OtherActor :type "Actor Object Reference") (OtherComp :type "PrimitiveComponent Object Reference") (OtherBodyIndex :type Integer) (bFromSweep :type Boolean) (SweepResult :type "HitResult Structure (by ref)"))
  (if (== OtherActor (`self.PlayerRef`))
    (`KismetSystemLibrary.PrintString` "Got em")
    (`/Game/Player/BP_Player.GainPickup` (`self.PlayerRef`))
    (`self.K2_DestroyActor`)))

(fn `UserConstructionScript`)