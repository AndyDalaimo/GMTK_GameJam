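; Launch direction indicator actor that shows an Arrow at the player's LaunchDir component.
; It caches BP_Player on BeginPlay, then each Tick moves the Arrow there with fixed yaw and pitch taken from AngleOf2DVector.
; AngleOf2DVector holds a clamped arctangent of the mouse drag from the player's InitMousePos, but that calculation is not connected to any output.
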(event `self.ReceiveBeginPlay`
  (bind _returnvalue (`GameplayStatics.GetActorOfClass` "/Game/Player/BP_Player.BP_Player_C"))
  (set `self.PlayerRef` _returnvalue))

(event `self.ReceiveTick`
  (params (DeltaSeconds :type "Float (single-precision)"))
  (`SceneComponent.K2_SetWorldLocationAndRotation` (`self.Arrow`) (`SceneComponent.K2_GetComponentLocation` (`/Game/Player/BP_Player.LaunchDir` (`self.PlayerRef`))) (`KismetMathLibrary.MakeRotator` 0.0 (`self.AngleOf2DVector`) 90.0) false false))

(fn `UserConstructionScript`)