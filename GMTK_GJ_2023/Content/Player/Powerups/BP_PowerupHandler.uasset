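; Powerup carrier actor that slides horizontally with the mouse and can drop spray powerups.
; Each tick it teleports its Cube along world Y from mouse screen X plus the player's Y, less an offset, keeping X and Z fixed.
; It also turns its sprite to match mouse movement direction by comparing against the last stored X.
; DropPowerup spawns a BP_SprayPowerup at the Cube's location but is not called within this Blueprint.
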(event `self.ReceiveBeginPlay`
  (bind _returnvalue (`GameplayStatics.GetActorOfClass` "/Game/Player/BP_Player.BP_Player_C"))
  (set `self.PlayerRef` _returnvalue))

(event `self.ReceiveTick`
  (params (DeltaSeconds :type "Float (single-precision)"))
  (`self.Lock Position to XMouse`)
  (`self.FlipSprite`))

(fn `DropPowerup`
  (bind (_returnvalue_x _returnvalue_y _returnvalue_z) (`KismetMathLibrary.BreakVector` (`SceneComponent.K2_GetComponentLocation` (`self.Cube`))))
  (`|SpawnActorFromClass` "/Game/Player/Powerups/BP_SprayPowerup.BP_SprayPowerup_C" (`KismetMathLibrary.MakeTransform` (`KismetMathLibrary.MakeVector` _returnvalue_x _returnvalue_y _returnvalue_z)) "Undefined" "OverrideRootScale" null null))

(fn `FlipSprite`
  (if (< (`PlayerController.GetMousePosition` (`GameplayStatics.GetPlayerController` 0)) (`self.MouseXPos`))
    (`SceneComponent.K2_SetWorldRotation` (`self.Sprite`) (struct :`Yaw` -90.0) false false)
    (set `self.MouseXPos` (`PlayerController.GetMousePosition` (`GameplayStatics.GetPlayerController` 0)) :!label _label)
    (elif (> (`PlayerController.GetMousePosition` (`GameplayStatics.GetPlayerController` 0)) (`self.MouseXPos`))
      (`SceneComponent.K2_SetWorldRotation` (`self.Sprite`) (struct :`Yaw` 90.0) false false)
      (goto _label))))

(fn `Lock Position to XMouse`
  (bind (_returnvalue_x _returnvalue_y) (`KismetMathLibrary.BreakVector` (`SceneComponent.K2_GetComponentLocation` (`/Game/Player/BP_Player.Cube` (`self.PlayerRef`)))))
  (`SceneComponent.K2_SetWorldLocation` (`self.Cube`) (`KismetMathLibrary.MakeVector` 850.0 (- (+ (`PlayerController.GetMousePosition` (`GameplayStatics.GetPlayerController` 0)) _returnvalue_y) (`self.YOffset`)) 70.0) false true))

(fn `UserConstructionScript`)